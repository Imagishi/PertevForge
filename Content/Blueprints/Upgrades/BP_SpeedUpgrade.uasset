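; Speed upgrade Blueprint that raises the owning character's maximum fly speed.
; When the upgrade level changes, OnUpgraded selects a multiplier for the new level and applies it to the CharacterMovement MaxFlySpeed.
; The multiplier scales the current speed rather than a stored base value, so successive upgrades compound.
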(event `self.OnUpgraded`
  (params (NewUpgradeLevel :type Integer))
  (bind _charactermovement (`Character.CharacterMovement` (`self.GetOwningCharacter`)))
  (set `CharacterMovementComponent.MaxFlySpeed` (* (select `int` NewUpgradeLevel :`0` 1.0 :`1` 1.2 :`2` 1.2 :`3` 1.4 :`4` 1.4 :`5` 1.5) (`CharacterMovementComponent.MaxFlySpeed` _charactermovement)) _charactermovement))

(fn `UserConstructionScript`
  (`parent.UserConstructionScript`))