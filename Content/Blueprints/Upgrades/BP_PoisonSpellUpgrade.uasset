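; Upgrade Blueprint that grants and strengthens the poison spell as its upgrade level rises.
; On upgrade, level 1 spawns a BP_PoisonSpell actor at the world origin.
; Every upgrade then finds that actor with GetActorOfClass and sets its Multiplier from a per-level Select, which increases linearly with level.
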(event `self.OnUpgraded`
  (params (NewUpgradeLevel :type Integer))
  (`|ExecutionSequence`
    (:`then_0`
      (if (== NewUpgradeLevel 1)
        (`|SpawnActorFromClass` "/Game/Blueprints/Attacks/Spells/Varieties/BP_PoisonSpell.BP_PoisonSpell_C" (`KismetMathLibrary.Conv_VectorToTransform` (0.0 0.0 0.0)) "Undefined" "MultiplyWithRoot" null null)))
    (:`then_1`
      (bind _returnvalue (`GameplayStatics.GetActorOfClass` "/Game/Blueprints/Attacks/Spells/Varieties/BP_PoisonSpell.BP_PoisonSpell_C"))
      (set `/Game/Blueprints/Attacks/Spells/Varieties/BP_PoisonSpell.Multiplier` (select `int` NewUpgradeLevel :`0` 1.0 :`1` 1.4 :`2` 1.8 :`3` 2.2 :`4` 2.6 :`5` 3.0) _returnvalue))))

(fn `UserConstructionScript`
  (`parent.UserConstructionScript`))