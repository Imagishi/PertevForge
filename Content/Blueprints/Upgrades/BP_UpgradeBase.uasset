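; BP_UpgradeBase is a base actor Blueprint for player upgrades, meant to be subclassed by each upgrade type.
; Upgrade increments UpgradeLevel while it is below 5 and passes the result to OnUpgraded.
; Child classes override OnUpgraded for their effects; the base version only prints a "not implemented" message with object name and level.
; GetOwningCharacter returns player pawn 0 cast to BP_Player.
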(event `self.ReceiveBeginPlay`)

(event `self.ReceiveTick`
  (params (DeltaSeconds :type "Float (single-precision)")))

(event `Upgrade`
  ;[1 1 1] Upgrade yapmak için bunu çağıracağız
  (if (< (`self.UpgradeLevel`) 5)
    (bind _result (`/Engine/EditorBlueprintResources/StandardMacros.IncrementInt` (`self.UpgradeLevel`))
      (:`  `
        (`self.OnUpgraded` _result)))))

(event `OnUpgraded`
  (params (NewUpgradeLevel :type Integer))
  ;[1 1 1] Diğer upgrade class'larında bu kısımda upgrade sonucu olacak olayları yapıcaz
  (`KismetSystemLibrary.PrintText` (`|FormatText` "Upgrade Not Implemented! {u} upgraded to Level {level}" (`KismetSystemLibrary.GetObjectName` self) NewUpgradeLevel) true true (struct :`R` 1.0 :`A` 1.0) 11.0))

(fn `GetOwningCharacter`
  (returns (ReturnValue :type "/Game/Blueprints/Player/BP_Player Object Reference"))
  (return (cast `/Game/Blueprints/Player/BP_Player` (`GameplayStatics.GetPlayerPawn` 0) :!pure true)))

(fn `UserConstructionScript`)