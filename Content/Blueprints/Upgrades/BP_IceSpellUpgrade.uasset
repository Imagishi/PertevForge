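; Upgrade Blueprint for the ice spell that sets the spell's strength according to its upgrade level.
; On each OnUpgraded event it spawns a BP_IceSpell at the world origin, with no check for an existing one.
; It then looks the spell up with GetActorOfClass, rather than using the spawned reference, and sets that actor's Multiplier from a per-level Select.
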(event `self.OnUpgraded`
  (params (NewUpgradeLevel :type Integer))
  (`|SpawnActorFromClass` "/Game/Blueprints/Attacks/Spells/Varieties/BP_IceSpell.BP_IceSpell_C" (`KismetMathLibrary.Conv_VectorToTransform` (0.0 0.0 0.0)) "Undefined" "MultiplyWithRoot" null null)
  (bind _returnvalue (`GameplayStatics.GetActorOfClass` "/Game/Blueprints/Attacks/Spells/Varieties/BP_IceSpell.BP_IceSpell_C"))
  (set `/Game/Blueprints/Attacks/Spells/Varieties/BP_IceSpell.Multiplier` (select `int` NewUpgradeLevel :`0` 1.0 :`1` 1.3 :`2` 1.4 :`3` 1.4 :`4` 1.5 :`5` 1.5) _returnvalue))

(fn `UserConstructionScript`
  (`parent.UserConstructionScript`))