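; BP_Player is a Paper2D player pawn that moves along world X and Z and picks up items.
; It registers the IMC_Player Enhanced Input context on BeginPlay and feeds the move actions into movement input.
; Sideways input also turns the control rotation to face left or right, while Tick switches run and idle flipbooks by velocity.
; The E key action destroys overlapping BP_Item actors without storing them.
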(event `self.ReceiveBeginPlay`
  ;[0 0 0] Assigning Input Mapping Context
  (bind _asplayer_controller (cast `PlayerController` (`self.GetController`)))
  (`EnhancedInputSubsystemInterface.AddMappingContext` (pcsubsystem `EnhancedInputLocalPlayerSubsystem` _asplayer_controller) "/Game/Inputs/IMC_Player.IMC_Player" 0 (struct)))

(event `self.ReceiveTick`
  (params (DeltaSeconds :type "Float (single-precision)"))
  ;[0 0 0] Animations
  (if (> (`KismetMathLibrary.VSize` (`self.GetVelocity`)) 0.0)
    (`PaperFlipbookComponent.SetFlipbook` (`self.Sprite`) "/Game/2D_Assets/Character/Flipbooks/FB_Player_Run.FB_Player_Run")
    (else
      (`PaperFlipbookComponent.SetFlipbook` (`self.Sprite`) "/Game/2D_Assets/Character/Flipbooks/FB_Player_Idle.FB_Player_Idle"))))

(event `EnhancedInput|/Game/Inputs/Actions/IA_Move_Vertical`
  (params (ActionValue :type "Float (double-precision)") (ElapsedSeconds :type "Float (double-precision)") (TriggeredSeconds :type "Float (double-precision)") (InputAction :type "InputAction Object Reference" :default "/Game/Inputs/Actions/IA_Move_Vertical.IA_Move_Vertical"))
  ;[0 0 0] Movement Functions
  (:`Triggered`
    (`self.AddMovementInput` (0.0 0.0 1.0) ActionValue)))

(event `EnhancedInput|/Game/Inputs/Actions/IA_Move_Sideways`
  (params (ActionValue :type "Float (double-precision)") (ElapsedSeconds :type "Float (double-precision)") (TriggeredSeconds :type "Float (double-precision)") (InputAction :type "InputAction Object Reference" :default "/Game/Inputs/Actions/IA_Move_Sideways.IA_Move_Sideways"))
  ;[0 0 0] Movement Functions
  (:`Triggered`
    (`self.AddMovementInput` (1.0 0.0 0.0) ActionValue)
    (`Controller.SetControlRotation` (`self.GetController`) (select `bool` (> ActionValue 0.0) :`false` (`KismetMathLibrary.MakeRotator` 0.0 0.0 180.0) :`true` (`KismetMathLibrary.MakeRotator` 0.0)))))

(event `EnhancedInput|/Game/Inputs/Actions/IA_EKeyAction`
  (params (ActionValue :type Boolean) (ElapsedSeconds :type "Float (double-precision)") (TriggeredSeconds :type "Float (double-precision)") (InputAction :type "InputAction Object Reference" :default "/Game/Inputs/Actions/IA_EKeyAction.IA_EKeyAction"))
  (bind _overlappingactors (`self.GetOverlappingActors` "/Game/Blueprints/Item/BP_Item.BP_Item_C"))
  ;[0 0 0] Pickup Function
  (:`Triggered`
    (if (`KismetArrayLibrary.Array_IsNotEmpty` _overlappingactors)
      (`self.K2_DestroyActor` _overlappingactors))))

(fn `UserConstructionScript`)