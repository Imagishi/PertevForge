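; Status effect component for BP_Enemy that applies timed slow, burn and poison, each with a sprite tint.
; Slow lowers Velocity, while burn and poison run looping timers that deal periodic damage.
; Each call increments that effect's counter, then a Delay precedes the decrement and a reset at zero.
; Calls during a pending Delay add no matching decrement, and any reset whitens the sprite regardless of other effects.
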(event `ApplySlow`
  (params (Duration :type "Float (double-precision)" :default 3.0))
  (bind _returnvalue (`self.GetOwningEnemy`))
  (bind _returnvalue_2 (`self.GetOwningEnemy`))
  (bind _slow (`self.Slow`))
  (`/Engine/EditorBlueprintResources/StandardMacros.IncrementInt` (`self.Slow`)
    (:`  `
      (set `/Game/Blueprints/Enemies/BP_Enemy.Velocity` 0.025 _returnvalue_2)
      (`PaperFlipbookComponent.SetSpriteColor` (`PaperCharacter.Sprite` _returnvalue_2) (struct :`R` 0.085417 :`G` 0.578591 :`B` 1.0 :`A` 1.0))
      (`KismetSystemLibrary.Delay` Duration)
      (`/Engine/EditorBlueprintResources/StandardMacros.DecrementInt` _slow
        (:`  `
          (`/Engine/EditorBlueprintResources/StandardMacros.CompareInt` _slow
            (:`==`
              (set `/Game/Blueprints/Enemies/BP_Enemy.Velocity` 0.05 _returnvalue)
              (`PaperFlipbookComponent.SetSpriteColor` (`PaperCharacter.Sprite` _returnvalue) (struct :`R` 1.0 :`G` 1.0 :`B` 1.0 :`A` 1.0)))))))))

(event `ApplyBurn`
  (params (Duration :type "Float (single-precision)" :default 3.0))
  (`/Engine/EditorBlueprintResources/StandardMacros.IncrementInt` (`self.Burn`)
    (:`  `
      (bind _returnvalue (`KismetSystemLibrary.K2_SetTimerDelegate` (delegate `BurnEnemy`) 0.5 true))
      (`PaperFlipbookComponent.SetSpriteColor` (`PaperCharacter.Sprite` (`self.GetOwningEnemy`)) (struct :`R` 1.0 :`G` 0.071869 :`B` 0.028085 :`A` 1.0))
      (`KismetSystemLibrary.Delay` Duration)
      (bind _result (`/Engine/EditorBlueprintResources/StandardMacros.DecrementInt` (`self.Burn`))
        (:`  `
          (`/Engine/EditorBlueprintResources/StandardMacros.CompareInt` _result
            (:`==`
              (`PaperFlipbookComponent.SetSpriteColor` (`PaperCharacter.Sprite` (`self.GetOwningEnemy`)) (struct :`R` 1.0 :`G` 1.0 :`B` 1.0 :`A` 1.0))
              (`KismetSystemLibrary.K2_ClearAndInvalidateTimerHandle` _returnvalue))))))))

(event `BurnEnemy`
  (`GameplayStatics.ApplyDamage` (`self.GetOwningEnemy`) 3.0))

(event `ApplyPoison`
  (params (Duration :type "Float (single-precision)" :default 3.0))
  (`/Engine/EditorBlueprintResources/StandardMacros.IncrementInt` (`self.Poison`)
    (:`  `
      (bind _returnvalue (`KismetSystemLibrary.K2_SetTimerDelegate` (delegate `PoisonEnemy`) 0.2 true))
      (`PaperFlipbookComponent.SetSpriteColor` (`PaperCharacter.Sprite` (`self.GetOwningEnemy`)) (struct :`R` 0.130628 :`G` 0.004158 :`B` 1.0 :`A` 1.0))
      (`KismetSystemLibrary.Delay` Duration)
      (bind _result (`/Engine/EditorBlueprintResources/StandardMacros.DecrementInt` (`self.Poison`))
        (:`  `
          (`/Engine/EditorBlueprintResources/StandardMacros.CompareInt` _result
            (:`==`
              (`PaperFlipbookComponent.SetSpriteColor` (`PaperCharacter.Sprite` (`self.GetOwningEnemy`)) (struct :`R` 1.0 :`G` 1.0 :`B` 1.0 :`A` 1.0))
              (`KismetSystemLibrary.K2_ClearAndInvalidateTimerHandle` _returnvalue))))))))

(event `PoisonEnemy`
  (`GameplayStatics.ApplyDamage` (`self.GetOwningEnemy`) 0.5))

(fn `GetOwningEnemy`
  (returns (ReturnValue :type "/Game/Blueprints/Enemies/BP_Enemy Object Reference"))
  (return (cast `/Game/Blueprints/Enemies/BP_Enemy` (`self.GetOwner`) :!pure true)))

(fn `Print Slow`
  (params (A :type String))
  (`KismetSystemLibrary.PrintString` (`KismetStringLibrary.Concat_StrStr` A (`KismetStringLibrary.Conv_IntToString` (`self.Slow`))) true true (struct :`R` 1.0 :`B` 0.042548 :`A` 1.0) 9999.0))