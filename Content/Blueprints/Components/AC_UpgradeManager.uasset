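; AC_UpgradeManager is a component that provides the game's upgrade pool and random selections from it.
; On BeginPlay it spawns one actor for each StartupUpgrades class at the world origin.
; GetRandomUpgrades draws classes until it has three unique ones, then returns the spawned actor of each via GetActorOfClass.
; The draw only runs when the pool holds more than three classes.
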(event `self.ReceiveBeginPlay`
  (`self.GiveStartupUpgrades`))

(fn `GetRandomUpgrades`
  (returns (ReturnValue :type "Array of /Game/Blueprints/Upgrades/BP_UpgradeBase Object Reference"))
  (bind _randomupgrades (`self.RandomUpgrades`))
  (if (> (`KismetArrayLibrary.Array_Length` (`self.StartupUpgrades`)) 3)
    (`KismetArrayLibrary.Array_Clear` (`self.SelectedClasses`))
    (`KismetArrayLibrary.Array_Clear` (`self.RandomUpgrades`))
    (while (< (`KismetArrayLibrary.Array_Length` (`self.SelectedClasses`)) 3)
      (`KismetArrayLibrary.Array_AddUnique` (`self.SelectedClasses`) (`KismetArrayLibrary.Array_Random` (`self.StartupUpgrades`))))
    (for _array_element (`self.SelectedClasses`)
      (bind _returnvalue (`GameplayStatics.GetActorOfClass` _array_element))
      (`KismetArrayLibrary.Array_Add` _randomupgrades _returnvalue))
    (return _randomupgrades)))

(fn `GiveStartupUpgrades`
  (for _array_element (`self.StartupUpgrades`)
    (`|SpawnActorFromClass` _array_element (`KismetMathLibrary.Conv_VectorToTransform` (0.0 0.0 0.0)) "Undefined" "MultiplyWithRoot" null null)))