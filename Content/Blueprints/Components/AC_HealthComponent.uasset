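; AC_HealthComponent is an actor component that tracks its owner's health and signals death.
; On BeginPlay it resets Health to DefaultHealth and binds to the owner's OnTakeAnyDamage, routing incoming damage into DealDamage.
; DealDamage ignores hits once dead, clamps Health at zero and broadcasts OnDeath when health runs out.
; IsAlive and GetNormalizedHealth expose the alive state and the health fraction relative to DefaultHealth.
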(event `self.ReceiveBeginPlay`
  (set `self.Health` (`self.DefaultHealth`))
  (add `Actor.OnTakeAnyDamage` (`self.GetOwner`) (`|CreateDelegate` :!event `OnTakeAnyDamage_Event`)))

(event `OnTakeAnyDamage_Event`
  (params (DamagedActor :type "Actor Object Reference") (Damage :type "Float (single-precision)") (DamageType :type "DamageType Object Reference") (InstigatedBy :type "Controller Object Reference") (DamageCauser :type "Actor Object Reference"))
  (`self.DealDamage` Damage))

(fn `DealDamage`
  (params (InDamage :type "Float (double-precision)"))
  (if (`self.IsAlive`)
    (set `self.Health` (`KismetMathLibrary.FMax` (- (`self.Health`) (`local.InDamage`))))
    (if (not (`self.IsAlive`))
      (`self.OnDeath`))))

(fn `GetNormalizedHealth`
  (returns (ReturnValue :type "Float (double-precision)"))
  (return (/ (`self.Health`) (`self.DefaultHealth`))))

(fn `IsAlive`
  (returns (ReturnValue :type Boolean))
  (return (> (`self.Health`) 0.0)))