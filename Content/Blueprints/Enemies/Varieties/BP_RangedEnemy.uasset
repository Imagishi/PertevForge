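; Ranged enemy variant that halts when the player is within close range and repeatedly fires projectile-style attacks at them.
; Tick checks distance to BP_Player, stopping movement and using a DoOnce to start a looping AttackPlayer timer.
; Moving out of range clears the timer and resets the DoOnce.
; AttackPlayer spawns BP_EnemyRangedAttack at the enemy's location, rotated toward the player via look-at and RInterpTo.
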(event `self.ReceiveBeginPlay`
  (`parent.ReceiveBeginPlay`))

(event `self.ReceiveTick`
  (params (DeltaSeconds :type "Float (single-precision)"))
  (bind _charactermovement (`self.CharacterMovement`))
  (`parent.ReceiveTick` DeltaSeconds)
  (bind _returnvalue (`GameplayStatics.GetActorOfClass` "/Game/Blueprints/Player/BP_Player.BP_Player_C"))
  (if (> (`KismetMathLibrary.Vector_Distance` (`self.K2_GetActorLocation` _returnvalue) (`self.K2_GetActorLocation`)) 200.0)
    (`KismetSystemLibrary.K2_ClearTimer` null "AttackPlayer")
    (goto _label :!via `Reset`)
    (else
      (`/Engine/EditorBlueprintResources/StandardMacros.IsValid` _charactermovement
        (:`Is Valid`
          (`MovementComponent.StopMovementImmediately` _charactermovement)
          (`/Engine/EditorBlueprintResources/StandardMacros.DoOnce` false :!label _label
            (:`Completed`
              (`KismetSystemLibrary.K2_SetTimer` null "AttackPlayer" 2.0 true))))))))

(fn `AttackPlayer`
  (bind _returnvalue (`GameplayStatics.GetActorOfClass` "/Game/Blueprints/Player/BP_Player.BP_Player_C"))
  (`|SpawnActorFromClass` "/Game/Blueprints/Attacks/EnemyAttacks/BP_EnemyRangedAttack.BP_EnemyRangedAttack_C" (`KismetMathLibrary.MakeTransform` (`self.K2_GetActorLocation`) (`KismetMathLibrary.RInterpTo` (`self.K2_GetActorRotation`) (`KismetMathLibrary.FindLookAtRotation` (`self.K2_GetActorLocation`) (`self.K2_GetActorLocation` _returnvalue)) (`GameplayStatics.GetWorldDeltaSeconds`)) (`self.GetActorScale3D`)) "AlwaysSpawn" "MultiplyWithRoot" null null))

(fn `UserConstructionScript`
  (`parent.UserConstructionScript`))