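; BP_Enemy is a flying enemy that chases BP_Player and deals contact damage.
; Each tick it aims an arrow at the player and adds movement input toward them, then destroys itself once Health is depleted.
; Incoming damage reduces Health.
; Capsule overlap with the player starts a looping timer that applies damage repeatedly, and ending the overlap clears it.
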(event `self.ReceiveBeginPlay`
  (`CharacterMovementComponent.SetMovementMode` (`self.CharacterMovement`) "MOVE_Flying" 0))

(event `self.ReceiveTick`
  (params (DeltaSeconds :type "Float (single-precision)"))
  (`|ExecutionSequence`
    (:`then_0`
      (bind _returnvalue (`GameplayStatics.GetActorOfClass` "/Game/Blueprints/Player/BP_Player.BP_Player_C"))
      (bind _returnvalue_2 (`KismetMathLibrary.FindLookAtRotation` (`self.K2_GetActorLocation`) (`self.K2_GetActorLocation` _returnvalue)))
      (`SceneComponent.K2_SetWorldRotation` (`self.Arrow1`) _returnvalue_2 false false)
      (`self.AddMovementInput` (`KismetMathLibrary.GetForwardVector` _returnvalue_2) 0.05))
    (:`then_1`
      (if (<= (`self.Health`) 0.0)
        (`self.K2_DestroyActor`)))))

(event `self.ReceiveAnyDamage`
  (params (Damage :type "Float (single-precision)") (DamageType :type "DamageType Object Reference") (InstigatedBy :type "Controller Object Reference") (DamageCauser :type "Actor Object Reference"))
  (set `self.Health` (- (`self.Health`) Damage)))

(event `self.CapsuleComponent.OnComponentBeginOverlap`
  (params (OverlappedComponent :type "PrimitiveComponent Object Reference") (OtherActor :type "Actor Object Reference") (OtherComp :type "PrimitiveComponent Object Reference") (OtherBodyIndex :type Integer) (bFromSweep :type Boolean) (SweepResult :type "HitResult Structure (by ref)"))
  (cast `/Game/Blueprints/Player/BP_Player` OtherActor)
  (`KismetSystemLibrary.K2_SetTimer` null "Apply Damage Event" 0.1 true))

(event `self.CapsuleComponent.OnComponentEndOverlap`
  (params (OverlappedComponent :type "PrimitiveComponent Object Reference") (OtherActor :type "Actor Object Reference") (OtherComp :type "PrimitiveComponent Object Reference") (OtherBodyIndex :type Integer))
  (cast `/Game/Blueprints/Player/BP_Player` OtherActor)
  (`KismetSystemLibrary.K2_ClearTimer` null "Apply Damage Event"))

(fn `Apply Damage Event`
  (bind _returnvalue (`GameplayStatics.GetActorOfClass` "/Game/Blueprints/Player/BP_Player.BP_Player_C"))
  (`GameplayStatics.ApplyDamage` _returnvalue 3.0))

(fn `UserConstructionScript`)