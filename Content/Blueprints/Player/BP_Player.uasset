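; Player character for a 2D game, moved on the X/Z plane with flipbook run/idle animation and automatic weapon attacks.
; BeginPlay sets up Enhanced Input, spawns startup spells and creates the HUD.
; Tick uses Delays to pace sword or bow attacks by weapon, with arrows aimed at the nearest BP_Enemy, if any.
; The E action destroys overlapping actors as pickup, and death reloads Main2D after a delay.
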(event `self.ReceiveBeginPlay`
  ;[0 0 0] Assigning Input Mapping Context
  (bind _asplayer_controller (cast `PlayerController` (`self.GetController`)))
  (`EnhancedInputSubsystemInterface.AddMappingContext` (pcsubsystem `EnhancedInputLocalPlayerSubsystem` _asplayer_controller) "/Game/Inputs/IMC_Player.IMC_Player" 0 (struct))
  (for _array_element (`self.StartupSpells`)
    (`|SpawnActorFromClass` _array_element (`KismetMathLibrary.Conv_VectorToTransform` (0.0 0.0 0.0)) "Undefined" "MultiplyWithRoot" null null))
  (bind _returnvalue (`|CreateWidget` "/Game/UI/WB_HUD.WB_HUD_C"))
  (`UserWidget.AddToViewport` _returnvalue 0))

(event `EnhancedInput|/Game/Inputs/Actions/IA_Move_Vertical`
  (params (ActionValue :type "Float (double-precision)") (ElapsedSeconds :type "Float (double-precision)") (TriggeredSeconds :type "Float (double-precision)") (InputAction :type "InputAction Object Reference" :default "/Game/Inputs/Actions/IA_Move_Vertical.IA_Move_Vertical"))
  ;[0 0 0] Movement Functions
  (:`Triggered`
    (`self.AddMovementInput` (0.0 0.0 1.0) ActionValue)))

(event `self.HealthComponent.OnDeath`
  (`KismetSystemLibrary.Delay` 2.0)
  (`GameplayStatics.OpenLevel` "Main2D") ; Restarts map on death
)

(event `EnhancedInput|/Game/Inputs/Actions/IA_Move_Sideways`
  (params (ActionValue :type "Float (double-precision)") (ElapsedSeconds :type "Float (double-precision)") (TriggeredSeconds :type "Float (double-precision)") (InputAction :type "InputAction Object Reference" :default "/Game/Inputs/Actions/IA_Move_Sideways.IA_Move_Sideways"))
  (bind _returnvalue (> ActionValue 0.0))
  (:`Triggered`
    (`self.AddMovementInput` (1.0 0.0 0.0) ActionValue)
    ;[0 0 0] Rotation
    (set `self.IsLookingRight` _returnvalue)
    (`Controller.SetControlRotation` (`self.GetController`) (select `bool` _returnvalue :`false` (`KismetMathLibrary.MakeRotator` 0.0 0.0 180.0) :`true` (`KismetMathLibrary.MakeRotator` 0.0)))))

(event `self.ReceiveTick`
  (params (DeltaSeconds :type "Float (single-precision)"))
  (`|ExecutionSequence`
    (:`then_0`
      ;[0 0 0] Movement Animations
      (if (> (`KismetMathLibrary.VSize` (`self.GetVelocity`)) 0.0)
        (`PaperFlipbookComponent.SetFlipbook` (`self.Sprite`) "/Game/2D_Assets/Character/Flipbooks/FB_Player_Run.FB_Player_Run")
        (else
          (`PaperFlipbookComponent.SetFlipbook` (`self.Sprite`) "/Game/2D_Assets/Character/Flipbooks/FB_Player_Idle.FB_Player_Idle"))))
    (:`then_1`
      (switch `/Game/Enums/EStarterWeapon` (`self.PlayerWeapon`)
        (:`NewEnumerator0`
          (`KismetSystemLibrary.Delay` 2.0)
          (`self.SwordAttack`))
        (:`NewEnumerator1`
          (`KismetSystemLibrary.Delay` 2.0)
          (`self.ArrowAttack`))))))

(event `EnhancedInput|/Game/Inputs/Actions/IA_EKeyAction`
  (params (ActionValue :type Boolean) (ElapsedSeconds :type "Float (double-precision)") (TriggeredSeconds :type "Float (double-precision)") (InputAction :type "InputAction Object Reference" :default "/Game/Inputs/Actions/IA_EKeyAction.IA_EKeyAction"))
  (bind _overlappingactors (`self.GetOverlappingActors` null))
  ;[0 0 0] Pickup Function
  (:`Triggered`
    (if (`KismetArrayLibrary.Array_IsNotEmpty` _overlappingactors)
      (`self.K2_DestroyActor` _overlappingactors))))

(fn `ArrowAttack`
  (bind _nearestactor (`self.FindNearestEnemy`))
  (`/Engine/EditorBlueprintResources/StandardMacros.IsValid` _nearestactor
    (:`Is Valid`
      (`|SpawnActorFromClass` "/Game/Blueprints/Attacks/PlayerAttacks/BP_ArrowAttack.BP_ArrowAttack_C" (`KismetMathLibrary.MakeTransform` (`self.K2_GetActorLocation`) (`KismetMathLibrary.RInterpTo` (`self.K2_GetActorRotation`) (`KismetMathLibrary.FindLookAtRotation` (`self.K2_GetActorLocation`) (`self.K2_GetActorLocation` _nearestactor)) (`GameplayStatics.GetWorldDeltaSeconds`)) (`self.GetActorScale3D`)) "AlwaysSpawn" "MultiplyWithRoot" null null))
    (:`Is Not Valid`
      (`|SpawnActorFromClass` "/Game/Blueprints/Attacks/PlayerAttacks/BP_ArrowAttack.BP_ArrowAttack_C" (`KismetMathLibrary.MakeTransform` (`self.K2_GetActorLocation`) (`SceneComponent.K2_GetComponentRotation` (`self.Sprite`)) (`self.GetActorScale3D`)) "AlwaysSpawn" "MultiplyWithRoot" null null))))

(fn `Find Nearest Actor`
  (params (Class :type "Actor Class Reference") (`Target Location` :type "Vector Structure"))
  (returns (NearestActor :type "Actor Object Reference") (NearestDistance :type "Float (double-precision)"))
  (locals (Loc_NearestDistance :type "Float (double-precision)" :default 10000.0) (Loc_NearestActor :type "Actor Object Reference"))
  (bind _outactors (`GameplayStatics.GetAllActorsOfClass` Class))
  (for _array_element _outactors
    (bind _returnvalue (`KismetMathLibrary.Vector_Distance` (`self.K2_GetActorLocation` _array_element) (`local.Target Location`)))
    (if (< _returnvalue (`local.Loc_NearestDistance`))
      (set `local.Loc_NearestDistance` _returnvalue)
      (set `local.Loc_NearestActor` _array_element)))
  (return (`local.Loc_NearestActor`) (`local.Loc_NearestDistance`)))

(fn `FindNearestEnemy`
  (returns (NearestActor :type "Actor Object Reference") (NearestDistance :type "Float (double-precision)"))
  (bind (_nearestactor _nearestdistance) (`self.Find Nearest Actor` "/Game/Blueprints/Enemies/BP_Enemy.BP_Enemy_C" (`self.K2_GetActorLocation`)))
  (return _nearestactor _nearestdistance))

(fn `SwordAttack`
  (bind (_returnvalue_location _returnvalue_rotation _returnvalue_scale) (`KismetMathLibrary.BreakTransform` (`self.GetTransform`)))
  (`|SpawnActorFromClass` "/Game/Blueprints/Attacks/PlayerAttacks/BP_SwordAttack.BP_SwordAttack_C" (`KismetMathLibrary.MakeTransform` _returnvalue_location _returnvalue_rotation _returnvalue_scale) "AlwaysSpawn" "MultiplyWithRoot" null null))

(fn `UserConstructionScript`)