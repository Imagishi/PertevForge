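; BP_FireSpell is a spell variety that launches a fire projectile toward a targeted enemy when cast.
; On OnSpellCasted, it finds BP_Player and spawns BP_FireSpellProj at the player's location.
; The projectile's rotation comes from a single RInterpTo call between the spell actor's rotation and the look-at rotation from player to enemy.
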(event `self.OnSpellCasted`
  (params (`Casted Enemy` :type "Actor Object Reference"))
  (bind _returnvalue (`GameplayStatics.GetActorOfClass` "/Game/Blueprints/Player/BP_Player.BP_Player_C"))
  (bind _returnvalue_2 (`self.K2_GetActorLocation` _returnvalue))
  (`|SpawnActorFromClass` "/Game/Blueprints/Attacks/Spells/Varieties/Assets/FireSpell/BP_FireSpellProj.BP_FireSpellProj_C" (`KismetMathLibrary.MakeTransform` _returnvalue_2 (`KismetMathLibrary.RInterpTo` (`self.K2_GetActorRotation`) (`KismetMathLibrary.FindLookAtRotation` _returnvalue_2 (`self.K2_GetActorLocation` `Casted Enemy`)) (`GameplayStatics.GetWorldDeltaSeconds`))) "Undefined" "MultiplyWithRoot" null null))

(fn `UserConstructionScript`
  (`parent.UserConstructionScript`))