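; Projectile for the poison spell that damages and poisons the first enemy its hit box overlaps.
; On overlapping a BP_Enemy, it applies poison through the enemy's StatusEffectComponent, deals direct damage, then destroys itself.
; Both amounts scale with the Multiplier read from the first BP_PoisonSpell actor found in the world.
; It also destroys itself after a short lifetime.
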(event `self.ReceiveBeginPlay`
  (`KismetSystemLibrary.Delay` 3.0)
  (`self.K2_DestroyActor`))

(event `self.HitBox.OnComponentBeginOverlap`
  (params (OverlappedComponent :type "PrimitiveComponent Object Reference") (OtherActor :type "Actor Object Reference") (OtherComp :type "PrimitiveComponent Object Reference") (OtherBodyIndex :type Integer) (bFromSweep :type Boolean) (SweepResult :type "HitResult Structure (by ref)"))
  (bind _asbp_enemy (cast `/Game/Blueprints/Enemies/BP_Enemy` OtherActor))
  (bind _returnvalue (`GameplayStatics.GetActorOfClass` "/Game/Blueprints/Attacks/Spells/Varieties/BP_PoisonSpell.BP_PoisonSpell_C"))
  (bind _multiplier (`/Game/Blueprints/Attacks/Spells/Varieties/BP_PoisonSpell.Multiplier` _returnvalue))
  (`/Game/Blueprints/Components/AC_StatusEffectComponent.ApplyPoison` (`/Game/Blueprints/Enemies/BP_Enemy.StatusEffectComponent` _asbp_enemy) (* _multiplier 4.0))
  (`GameplayStatics.ApplyDamage` _asbp_enemy (* _multiplier 10.0))
  (`self.K2_DestroyActor`))

(fn `UserConstructionScript`)