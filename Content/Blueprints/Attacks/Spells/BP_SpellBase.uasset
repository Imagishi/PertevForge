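; BP_SpellBase is a base spell Blueprint that targets the enemy nearest the player.
; BeginPlay starts a looping timer at CooldownTime, apparently to drive automatic casting, and stores its handle in ElapsedCooldown.
; CastSpell gets BP_Player, saves its FindNearestEnemy result as CastedEnemy, draws a debug sphere there and calls OnSpellCasted.
; OnSpellCasted only prints the spell and enemy names here.
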(event `self.ReceiveBeginPlay`
  (bind _returnvalue (`KismetSystemLibrary.K2_SetTimerDelegate` (`|CreateDelegate` :!event `Cast Spell`) (`self.CooldownTime`) true))
  (set `self.Elapsed Cooldown` _returnvalue))

(event `Cast Spell`
  (bind _returnvalue (`GameplayStatics.GetActorOfClass` "/Game/Blueprints/Player/BP_Player.BP_Player_C"))
  (`/Engine/EditorBlueprintResources/StandardMacros.IsValid` _returnvalue
    (:`Is Valid`
      (bind _nearestactor (`/Game/Blueprints/Player/BP_Player.FindNearestEnemy` _returnvalue))
      (bind _output_get (set `self.Casted Enemy` _nearestactor))
      (`KismetSystemLibrary.DrawDebugSphere` (`self.K2_GetActorLocation` _output_get) 50.0 12 (struct :`R` 1.0 :`G` 1.0 :`B` 1.0 :`A` 1.0) 2.0)
      (`self.OnSpellCasted` _output_get))))

(event `OnSpellCasted`
  (params (`Casted Enemy` :type "Actor Object Reference"))
  (`KismetSystemLibrary.PrintString` (`KismetTextLibrary.Conv_TextToString` (`|FormatText` "{spell} Spell Casted on {enemy}" (`KismetSystemLibrary.GetDisplayName` self) (`KismetSystemLibrary.GetDisplayName` (`self.Casted Enemy`)))) true true (struct :`A` 1.0) 2.0 "0"))

(fn `UserConstructionScript`)