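; BP_FireSpell is a short-lived fire spell actor that damages characters it overlaps and destroys itself three seconds after spawning.
; On overlap it reads IsEnemy from a BP_RangedEnemy found in the level through GetActorOfClass, rather than from its own caster.
; That flag selects the target: when true it damages an overlapped BP_Player, otherwise it deals heavier damage to an overlapped BP_Enemy.
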(event `self.ReceiveBeginPlay`
  (`KismetSystemLibrary.Delay` 3.0)
  (`self.K2_DestroyActor`))

(event `self.ReceiveActorBeginOverlap`
  (params (OtherActor :type "Actor Object Reference"))
  (bind _returnvalue (`GameplayStatics.GetActorOfClass` "/Game/Blueprints/Enemies/Varieties/BP_RangedEnemy.BP_RangedEnemy_C"))
  (if (`/Game/Blueprints/Enemies/Varieties/BP_RangedEnemy.IsEnemy` _returnvalue)
    (bind _asbp_player (cast `/Game/Blueprints/Player/BP_Player` OtherActor))
    (`GameplayStatics.ApplyDamage` _asbp_player 20.0)
    (else
      (bind _asbp_enemy (cast `/Game/Blueprints/Enemies/BP_Enemy` OtherActor))
      (`GameplayStatics.ApplyDamage` _asbp_enemy 50.0))))

(fn `UserConstructionScript`
  (`parent.UserConstructionScript`))